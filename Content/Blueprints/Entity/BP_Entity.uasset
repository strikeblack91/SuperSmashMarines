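; BP_Entity is an entity Blueprint, apparently a shared base, that handles life and death for game actors.
; DecreaseLife subtracts damage unless IsFinished reports that GameStatement is in its finished state, and returns whether the hit depleted Life.
; At zero life or below, it casts self to BP_Meteorite to call DestroyMeteorite, and destroys any other entity directly.
; The event graph and construction script are empty.
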(event EventBeginPlay)

(event Collision|EventActorBeginOverlap
  (params (OtherActor :type Actor%20Object%20Reference)))

(event EventTick
  (params (DeltaSeconds :type Float%20%28single-precision%29)))

(fn ConstructionScript)

(fn DecreaseLife
  (params (Damage :type Integer))
  ;[1 1 1] Decrease life.
  (if (Math|Boolean|Equal(Boolean) (CallFunction|IsFinished) false)
    (Variables|Default|SetLife (- (Variables|Default|GetLife) Damage))
    ;[1 1 1] Destroy actor if no life left.
    (if (<= (Variables|Default|GetLife) 0)
      (bind _asbp_meteorite (Utilities|Casting|CastToBP_Meteorite self)
        (:then
          (Default|DestroyMeteorite _asbp_meteorite))
        (:CastFailed
          (Actor|DestroyActor)))
      (return true)
      (else
        (return false)))))

(fn IsFinished
  (if (Utilities|Enum|Equal(Enum) (Variables|Default|GetGameStatement) "NewEnumerator1")
    (return true)
    (else
      (return false))))