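; BP_ForWar is a moving hazard that damages BP_Entity actors it touches.
; While Activate is set and IsFinished is false, Tick calls UpdateLocation with the Arrow's forward vector, identically for Up and Down directions.
; Box overlaps call DecreaseLife with Damage on valid entities, also only until finished.
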(event OnComponentBeginOverlap(Box)
  (params (OverlappedComponent :type Primitive%20Component%20Object%20Reference) (OtherActor :type Actor%20Object%20Reference) (OtherComp :type Primitive%20Component%20Object%20Reference) (OtherBodyIndex :type Integer) (bFromSweep :type Boolean) (SweepResult :type Hit%20Result%20Structure%20%28by%20ref%29))
  (if (not (CallFunction|IsFinished))
    (bind _asbp_entity (Utilities|Casting|CastToBP_Entity OtherActor))
    (Utilities|IsValid _asbp_entity
      (:Is%20Valid
        (Default|DecreaseLife _asbp_entity (Variables|Default|GetDamage))))))

(event EventTick
  (params (DeltaSeconds :type Float%20%28single-precision%29))
  (bind _arrow (Variables|Default|GetArrow))
  (bind _returnvalue (Math|Vector|GetForwardVector _arrow))
  (|CallParentFunction DeltaSeconds)
  (if (not (CallFunction|IsFinished))
    (if (Variables|Default|GetActivate)
      (switch Utilities|FlowControl|Switch|SwitchonE_Direction (Variables|Default|GetDirection)
        (:NewEnumerator0
          (CallFunction|UpdateLocation _returnvalue))
        (:NewEnumerator1
          (CallFunction|UpdateLocation _returnvalue))))))

(fn ConstructionScript
  (|CallParentFunction))