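; BP_Projectile is a projectile entity that moves by direct location offsets and can change the player's projectile class.
; UpdateLocation shifts the actor along a given direction by Speed per call, without sweep or delta-time scaling.
; SetNewClassReferenceProjectile casts an entity to BP_Meteorite and copies its projectile class onto PlayerReference.
; The event graph has no logic of its own, with Tick only calling the parent.
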(event EventBeginPlay
  (|CallParentFunction) ; This node is disabled and will not be called.\nDrag off pins to build functionality.
)

(event Collision|EventActorBeginOverlap
  (params (OtherActor :type Actor%20Object%20Reference))
  (|CallParentFunction OtherActor) ; This node is disabled and will not be called.\nDrag off pins to build functionality.
)

(event EventTick
  (params (DeltaSeconds :type Float%20%28single-precision%29))
  (|CallParentFunction DeltaSeconds))

(fn ConstructionScript
  (|CallParentFunction))

(fn SetNewClassReferenceProjectile
  (params (Entity :type BP%20Entity%20Object%20Reference))
  (bind _asbp_meteorite (Utilities|Casting|CastToBP_Meteorite Entity))
  (Variables|/Game/Blueprints/Entity/BP_Player.BP_Player_C|SetClassReferenceProjectile (Variables|Default|GetPlayer_Reference) (Variables|/Game/Blueprints/Entity/BP_Meteorite.BP_Meteorite_C|GetClassReferenceProjectile _asbp_meteorite)))

(fn UpdateLocation
  (params (Direction :type Vector))
  (Transformation|SetActorLocation (+ (Transformation|GetActorLocation) (* Direction (Variables|Default|GetSpeed))) false false))