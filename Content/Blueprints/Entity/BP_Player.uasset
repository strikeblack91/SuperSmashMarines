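; BP_Player is the player's starship, which moves continuously along the Y axis and fires automatically.
; Tick moves it by Speed in the sign set by Direction, which ToggleDirection flips, and destroys it beyond fixed Y limits.
; A looping timer calls Shoot, which fires a single or triple shot along arrow components, passing each projectile a reference to the player.
; Movement and shooting stop once IsFinished is true.
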(event EventTick
  (params (DeltaSeconds :type Float%20%28single-precision%29))
  (|CallParentFunction DeltaSeconds)
  (CallFunction|UpdateLocationPlayer)
  (CallFunction|IsOutOfLimitation))

(event EventBeginPlay
  (CallFunction|SetSpeedShoot))

(fn ConstructionScript
  (|CallParentFunction))

(fn SetSpeedShoot
  (Utilities|Time|SetTimerbyFunctionName 0 "Shoot" (Variables|Default|GetSpeedShoot) true))

(fn ToggleDirection
  (bind _direction (Variables|Default|GetDirection))
  (if (Utilities|Enum|Equal(Enum) _direction "NewEnumerator0")
    (|SetBy-RefVar _direction "NewEnumerator1")
    (else
      (|SetBy-RefVar _direction "NewEnumerator0"))))

(fn UpdateLocationPlayer
  (bind _defaultsceneroot (Variables|Default|GetDefaultSceneRoot))
  (bind _returnvalue (Transformation|GetWorldLocation _defaultsceneroot))
  ;[1 1 1] Depending of the direction, we update the Pawn movement.
  (if (Math|Boolean|Equal(Boolean) (CallFunction|IsFinished) false)
    (if (Utilities|Enum|Equal(Enum) (Variables|Default|GetDirection) "NewEnumerator0")
      (Transformation|SetWorldLocation (Variables|Default|GetDefaultSceneRoot) (+ _returnvalue (Math|Vector|MakeVector 0.0 (Variables|Default|GetSpeed) 0.0)) false false)
      (else
        (Transformation|SetWorldLocation (Variables|Default|GetDefaultSceneRoot) (+ _returnvalue (Math|Vector|MakeVector 0.0 (* (Variables|Default|GetSpeed) -1.0) 0.0)) false false)))))

(fn Shoot
  (switch Utilities|FlowControl|Switch|SwitchonE_shootMod (Variables|Default|GetShootMod)
    (:NewEnumerator0
      (CallFunction|NormalShot (Variables|Default|GetMiddle)))
    (:NewEnumerator1
      (CallFunction|TripleShot))))

(fn IsOutOfLimitation
  (bind _returnvalue (Transformation|GetActorLocation))
  ;[1 1 1] If the player is out of the limit, he is destroyed.
  (if (>= (.y _returnvalue) 7.5e+02)
    (Actor|DestroyActor)
    (elif (<= (.y _returnvalue) -7.5e+02)
      (Actor|DestroyActor))))

(fn NormalShot
  (params (Arrow :type Arrow%20Component%20Object%20Reference))
  (if (Math|Boolean|Equal(Boolean) (CallFunction|IsFinished) false)
    (bind _returnvalue (Game|SpawnActorfromClass (Variables|Default|GetClassReferenceProjectile) (Math|Transform|MakeTransform (+ (Transformation|GetActorLocation) (* (Math|Vector|GetForwardVector Arrow) 2e+02)) (Math|Conversions|RotationFromXVector (Math|Vector|GetForwardVector Arrow))) "AlwaysSpawn" 0 0))
    ;[1 1 1] Security, it can crash here.
    (Utilities|IsValid _returnvalue
      (:Is%20Valid
        (Variables|/Game/Blueprints/Entity/BP_Projectile.BP_Projectile_C|SetPlayer_Reference _returnvalue self)))))

(fn TripleShot
  (CallFunction|NormalShot (Variables|Default|GetMiddle))
  (CallFunction|NormalShot (Variables|Default|GetUp))
  (CallFunction|NormalShot (Variables|Default|GetDown)))